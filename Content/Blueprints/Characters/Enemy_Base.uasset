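; Base enemy character that wanders and reacts to seen pawns through searching, alert and hostile attention states, each setting spotlight color and walk speed.
; A one-second looping timer runs the current state and a countdown that can drop hostile to alert.
; PawnSensing sets hostile, resets the countdown and stores the seen 0_Base pawn as move target.
; Wander points are random reachable locations, retried for facing angle and minimum distance, with optional debug trace.
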(event `self.ReceiveTick`
  (params (DeltaSeconds :type "Float (single-precision)"))
  ;[1 1 1] Change Var Default to Display Line Trace (or not)
  (`self.DisplayLineTraceToLocation` (`self.DisplayLineTraceToLocation?`)))

(event `MoveToRandomLocation`
  (bind _timecounter (`self.TimeCounter`))
  (set `self.TimeCounter` (- (`self.TimeCounter`) 1))
  (switch `int` (`self.AttentionMode`)
    (:`1`
      (`self.Status1_Searching`)
      (if (`self.reachedRandomizedLocation`)
        (set `self.reachedRandomizedLocation` false)
        (bind _targetlocation (`self.RandomizedMovement`))
        (`|AIMoveTo` self _targetlocation null
          (:`OnSuccess`
            (set `self.reachedRandomizedLocation` true)))))
    (:`2`
      (`self.Status2_Alert`)
      (if (`self.reachedLastKnownPosition`)
        (set `self.reachedLastKnownPosition` true)
        (bind _targetlocation_2 (`self.HostileMovement`))
        (`|AIMoveTo` self _targetlocation_2 null
          (:`OnSuccess`
            (set `self.reachedLastKnownPosition` true)
            (if (`self.reachedRandomizedLocation`)
              (set `self.reachedRandomizedLocation` false)
              (bind _targetlocation_3 (`self.RandomizedMovement`))
              (`|AIMoveTo` self _targetlocation_3 null
                (:`then`
                  (`KismetSystemLibrary.Delay` 1.0))
                (:`OnSuccess`
                  (set `self.reachedRandomizedLocation` true))))))))
    (:`3`
      (`self.Status3_Hostile`)
      (if (not (`self.reachedLastKnownPosition`))
        (bind _targetlocation_4 (`self.HostileMovement`))
        (`|AIMoveTo` self _targetlocation_4 null
          (:`then`
            (if (not (`self.reachedLastKnownPosition`))
              (`KismetSystemLibrary.PrintText` "Can't see the player" true true (struct :`R` 0.990895 :`B` 1.0 :`A` 1.0) 20.0)
              (`KismetSystemLibrary.PrintString` (`KismetStringLibrary.Concat_StrStr` "Time Counter:" (`KismetStringLibrary.Conv_IntToString` _timecounter)) true true (struct :`R` 0.122258 :`B` 1.0 :`A` 1.0) 20.0)
              (if (== _timecounter 5)
                _
                (elif (== (`self.TimeCounter`) 0)
                  (set `self.AttentionMode` 2)
                  (set `self.reachedLastKnownPosition` true)))))
          (:`OnSuccess`
            (set `self.reachedLastKnownPosition` true)))))))

(event `self.ReceiveBeginPlay`
  (`|ExecutionSequence`
    (:`then_0`
      (set `self.AttentionMode` 1)
      (`KismetSystemLibrary.K2_SetTimerDelegate` (delegate `MoveToRandomLocation`) 1.0 true))))

(event `self.PawnSensing.OnSeePawn`
  (params (Pawn :type "Pawn Object Reference"))
  (bind _as0_base (cast `/Game/Blueprints/Characters/0_Base` Pawn))
  (set `self.CanSeePlayer` true)
  (set `self.SeenPlayer` _as0_base)
  (set `self.AttentionMode` 3)
  (set `self.lastKnownLocation` (`CharacterMovementComponent.GetLastUpdateLocation` (`self.CharacterMovement`)))
  (set `self.TimeCounter` 5))

(fn `CountDownXSeconds`
  (params (MaxSeconds :type Integer))
  (returns (NewParam :type Boolean))
  (return (!= (- MaxSeconds 1) 0)))

(fn `DisplayLineTraceToLocation`
  (params (`DisplayLineTrace?` :type Boolean))
  (bind _returnvalue (`self.K2_GetActorLocation`))
  (if `DisplayLineTrace?`
    (`KismetSystemLibrary.LineTraceSingle` :`Start` _returnvalue :`End` (+ _returnvalue (* (`KismetMathLibrary.Conv_RotatorToVector` (`KismetMathLibrary.FindLookAtRotation` _returnvalue (`self.RandLocation`))) (`KismetMathLibrary.VSize` (- (`self.ActorLocation`) (`self.RandLocation`))))) :`TraceChannel` "TraceTypeQuery1" :`DrawDebugType` "ForOneFrame")))

(fn `GetAngleBetweenVectors`
  (returns (`LocationIsOK?` :type Boolean))
  (bind _returnvalue (- (`self.ActorRotation`) (`self.TargetRotation`)))
  (bind _returnvalue_2 (`KismetMathLibrary.VSize` (- (`self.ActorLocation`) (`self.RandLocation`))))
  (if (>= _returnvalue 0.0)
    (set `self.RotationDifference` _returnvalue)
    (else
      (set `self.RotationDifference` (* _returnvalue -1.0))))
  (if (<= (`self.RotationDifference`) (`self.MaxAngleDifference`))
    (if (>= _returnvalue_2 (`self.MinDistanceFromLocation`))
      ;[1 1 1] Logging of good results
      (`KismetSystemLibrary.PrintString` (`KismetStringLibrary.Concat_StrStr` "Ai found location distance: " (`KismetStringLibrary.Conv_DoubleToString` _returnvalue_2)) false true (struct :`G` 0.66 :`B` 1.0 :`A` 1.0) 20.0)
      (`KismetSystemLibrary.PrintString` (`KismetStringLibrary.Concat_StrStr` "Ai found a good angle: " (`KismetStringLibrary.Conv_DoubleToString` (`self.RotationDifference`))) false true (struct :`G` 0.66 :`B` 1.0 :`A` 1.0) 20.0)
      (return true)
      (else
        _)))
  (return false))

(fn `HostileMovement`
  (returns (TargetLocation :type "Vector Structure"))
  (return (`CharacterMovementComponent.GetLastUpdateLocation` (`Character.CharacterMovement` (`self.SeenPlayer`)))))

(fn `RandomizedMovement`
  (returns (TargetLocation :type "Vector Structure"))
  ;[1 1 1] Randomized Movement of the Enemy.
  (bind _output_get (set `self.ActorLocation` (`self.K2_GetActorLocation` self)))
  (set `self.RandLocation` (`NavigationSystemV1.K2_GetRandomReachablePointInRadius` _output_get (`self.RadiusOfMoveToLocationSearch`) null null) :!label _label)
  (set `self.ActorRotation` (.yaw (`self.K2_GetActorRotation` self)))
  (set `self.TargetRotation` (.yaw (`KismetMathLibrary.FindLookAtRotation` (`self.K2_GetActorLocation` self) (`self.RandLocation`))))
  ;[1 1 1] Checking generated location IF within angle difference scope and above min distance
  (bind _locationisok_ (`self.GetAngleBetweenVectors`))
  (if (not _locationisok_)
    (bind _output_get_2 (set `self.RandCounter` (+ (`self.RandCounter`) 1)))
    (if (>= _output_get_2 20)
      (`KismetSystemLibrary.PrintText` "Ai tried to find a location over 20 tries. Giving up" true true (struct :`G` 0.66 :`B` 1.0 :`A` 1.0) 20.0)
      (else
        (goto _label))))
  (set `self.RandCounter` 0)
  (return (`self.RandLocation`)))

(fn `Status1_Searching`
  (`LightComponent.SetLightColor` (`self.SpotLight`) (struct :`G` 0.390625 :`B` 0.020414 :`A` 1.0) true)
  (set `CharacterMovementComponent.MaxWalkSpeed` (`self.MovementSpeed`) (`self.CharacterMovement`))
  (`KismetSystemLibrary.PrintText` "Turned Pasive (Status 1)" true true (struct :`G` 0.66 :`B` 1.0 :`A` 1.0) 45.0))

(fn `Status2_Alert`
  (`LightComponent.SetLightColor` (`self.SpotLight`) (struct :`R` 0.911458 :`G` 0.747527 :`B` 0.05045 :`A` 1.0) true)
  (set `CharacterMovementComponent.MaxWalkSpeed` (* (`self.MovementSpeed`) 1.5) (`self.CharacterMovement`))
  (`KismetSystemLibrary.PrintText` "Turned Alert (Status 2)" true true (struct :`G` 0.66 :`B` 1.0 :`A` 1.0) 45.0))

(fn `Status3_Hostile`
  (`LightComponent.SetLightColor` (`self.SpotLight`) (struct :`R` 0.40625 :`B` 0.378856 :`A` 1.0) true)
  (set `CharacterMovementComponent.MaxWalkSpeed` (* (`self.MovementSpeed`) 1.5) (`self.CharacterMovement`))
  (`KismetSystemLibrary.PrintText` "Turned Hostile (status 3)" true true (struct :`G` 0.66 :`B` 1.0 :`A` 1.0) 45.0))

(fn `UserConstructionScript`)