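; Gameplay player controller that handles pause input and periodic progress saving during play.
; On BeginPlay it caches the GameInfoInstance and starts a looping timer that refreshes wave UI player info, saves progress through that instance and prints an autosave notice.
; The Menu input opens the pause menu through the game instance, and the P key increments the wave UI's enemies-left count.
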(event `self.ReceiveBeginPlay`
  (bind _asgame_info_instance (cast `/Game/Blueprints/AllLevels/GameInfoInstance` (`GameplayStatics.GetGameInstance`)))
  (set `self.GameInfoInstanceRef` _asgame_info_instance)
  (`KismetSystemLibrary.K2_SetTimer` null "AutosaveProgress" 60.0 true))

(event `InputAction|Menu`
  (params (Key :type "Key Structure"))
  (:`Pressed`
    (`/Game/Blueprints/AllLevels/GameInfoInstance.ShowPauseMenu` (`self.GameInfoInstanceRef`))))

(event `Key|P`
  (params (Key :type "Key Structure"))
  (bind _waveuiwb (`/Game/Blueprints/AllLevels/GameInfoInstance.WaveUIWB` (`self.GameInfoInstanceRef`)))
  ;[1 1 1] Increments Enemies Left in Wave Ui
  (:`Pressed`
    (set `/Game/UI/Wave/Wave_UI.EnemiesLeft` (+ (`/Game/UI/Wave/Wave_UI.EnemiesLeft` _waveuiwb) 1) _waveuiwb)))

(fn `AutosaveProgress`
  (bind _gameinfoinstanceref (`self.GameInfoInstanceRef`))
  (`/Game/UI/Wave/Wave_UI.UpdatePlayerInfo` (`/Game/Blueprints/AllLevels/GameInfoInstance.WaveUIWB` _gameinfoinstanceref))
  (`/Game/Blueprints/AllLevels/GameInfoInstance.SaveProgress` _gameinfoinstanceref)
  (`KismetSystemLibrary.PrintText` "Autosaved" true true (struct :`R` 0.352128 :`G` 1.0 :`B` 0.18964 :`A` 1.0) 10.0))

(fn `UserConstructionScript`)